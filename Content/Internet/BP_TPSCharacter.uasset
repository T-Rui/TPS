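; Third-person shooter character Blueprint handling weapon fire and damage.
; The "test" input calls Shoot and ShootNew, which spawns a projectile from the gun muzzle along control rotation, plays sound and decrements ammo, with its ammo check disconnected.
; ShootGrenad similarly launches grenades when equipped, aiming and stocked, but its only event-graph call is unreachable.
; AnyDamage lowers Health, clamped at zero, with no death handling.
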(event `self.ReceiveBeginPlay`)

(event `InputAction|test`
  (params (Key :type "Key Structure"))
  (:`Pressed`
    (`self.Shoot`)
    (`self.ShootNew`)))

(event `self.ReceiveAnyDamage`
  (params (Damage :type "Float (single-precision)") (DamageType :type "DamageType Object Reference") (InstigatedBy :type "Controller Object Reference") (DamageCauser :type "Actor Object Reference"))
  ;[1 1 1] Damage
  (set `self.health` (`KismetMathLibrary.FMax` (- (`self.health`) Damage)))
  (if true
    _))

(fn `ShootGrenad`
  (bind _pgun (`self.pGun`))
  (if (`self.bEquip`)
    (if (`self.bAim`)
      (if (> (`self.nCurrentGrenad`) 0)
        (`|SpawnActorFromClass` "/Game/BallisticsVFX/FXSpawnerBlueprints/Projectiles/Grenade_launched.Grenade_launched_C" (`KismetMathLibrary.MakeTransform` (`SceneComponent.GetSocketLocation` _pgun "Socket_Muzzle") (`self.GetControlRotation`)) "AdjustIfPossibleButDontSpawnIfColliding" "OverrideRootScale" null true null :!pinned true) ; Spawn projectile
        (`GameplayStatics.SpawnSoundAttached` "/Game/BallisticsVFX/SFX/GrenLauncher/GrenadeLauncher_cue.GrenadeLauncher_cue" _pgun "None" (0.0 0.0 0.0) (struct) "KeepRelativeOffset" false 1.0 1.0 0.0 null null)
        (set `self.nCurrentGrenad` (- (`self.nCurrentGrenad`) 1))))))

(fn `ShootNew`
  (bind _pgun (`self.pGun`))
  (if (`self.bEquip`)
    (`|SpawnActorFromClass` "/Game/BallisticsVFX/FXSpawnerBlueprints/Projectiles/CubitUniProjectile.CubitUniProjectile_C" (`KismetMathLibrary.MakeTransform` (`SceneComponent.GetSocketLocation` _pgun "Socket_Muzzle") (`self.GetControlRotation`)) "AdjustIfPossibleButDontSpawnIfColliding" "OverrideRootScale" null 30000.0 true true false "NewEnumerator1" 0 "NewEnumerator0" null :!pinned true) ; Spawn projectile
    (`GameplayStatics.SpawnSoundAttached` "/Game/BallisticsVFX/SFX/Guns/Rifle_fire.Rifle_fire" _pgun "None" (0.0 0.0 0.0) (struct) "KeepRelativeOffset" false 1.0 1.0 0.0 null null)
    (set `self.nCurrentAm` (- (`self.nCurrentAm`) 1))))

(fn `UserConstructionScript`)