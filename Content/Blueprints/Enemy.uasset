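; Enemy actor that takes two projectile hits to destroy and reports its death to the player character.
; The Hit event ignores non-projectile actors; the first projectile hit only sets the IsHit flag.
; The next hit plays explosion sound and particles at the hit location, destroys the actor, then calls KillNumEnemy on player 0's TPSCharacter.
; A local Killnum increment is left unconnected and never runs.
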(event `self.ReceiveHit`
  (params (MyComp :type "PrimitiveComponent Object Reference") (Other :type "Actor Object Reference") (OtherComp :type "PrimitiveComponent Object Reference") (bSelfMoved :type Boolean) (HitLocation :type "Vector Structure") (HitNormal :type "Vector Structure") (NormalImpulse :type "Vector Structure") (Hit :type "HitResult Structure (by ref)"))
  ;[1 1 1] 爆炸销毁
  (cast `projectile` Other)
  (if (`self.IsHit`)
    (`GameplayStatics.PlaySoundAtLocation` "/Game/StarterContent/Audio/Explosion01.Explosion01" HitLocation (struct) 1.0 1.0 0.0 null null null)
    (`GameplayStatics.SpawnEmitterAtLocation` "/Game/StarterContent/Particles/P_Explosion.P_Explosion" HitLocation)
    (`self.K2_DestroyActor`)
    (bind _astpscharacter (cast `TPSCharacter` (`GameplayStatics.GetPlayerCharacter` 0)))
    (`TPSCharacter.KillNumEnemy` _astpscharacter)
    (else
      (set `self.IsHit` true))))

(fn `UserConstructionScript`)