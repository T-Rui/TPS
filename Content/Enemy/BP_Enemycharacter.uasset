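; Enemy character Blueprint that senses the player, reacts to projectile hits and dies after repeated hits.
; PawnSensing writes a seen BP_TPSCharacter to the "Player" key on its Blackboard.
; CubitUniProjectile hits increment a counter and set the "Ishit" Blackboard flag.
; Once the counter reaches its threshold, the next hit decrements the player character's CurrentNum and destroys the enemy.
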(event `self.PawnSensing.OnSeePawn`
  (params (Pawn :type "Pawn Object Reference"))
  (bind _returnvalue (`AIBlueprintHelperLibrary.GetBlackboard` self))
  (bind _asbp_tpscharacter (cast `/Game/Internet/BP_TPSCharacter` Pawn))
  (`/Engine/EditorBlueprintResources/StandardMacros.IsValid` _returnvalue
    (:`Is Valid`
      (`BlackboardComponent.SetValueAsObject` _returnvalue "Player" _asbp_tpscharacter))))

(event `self.ReceiveHit`
  (params (MyComp :type "PrimitiveComponent Object Reference") (Other :type "Actor Object Reference") (OtherComp :type "PrimitiveComponent Object Reference") (bSelfMoved :type Boolean) (HitLocation :type "Vector Structure") (HitNormal :type "Vector Structure") (NormalImpulse :type "Vector Structure") (Hit :type "HitResult Structure (by ref)"))
  (bind _hitnum (`self.HitNum`))
  (bind _returnvalue (>= (`self.HItNum`) 1))
  (cast `/Game/BallisticsVFX/FXSpawnerBlueprints/Projectiles/CubitUniProjectile` Other)
  (if (>= _hitnum 5)
    (bind _asbp_tpscharacter (cast `/Game/Internet/BP_TPSCharacter` (`GameplayStatics.GetPlayerCharacter` 0)))
    (set `/Game/Internet/BP_TPSCharacter.CurrentNum` (- (`/Game/Internet/BP_TPSCharacter.CurrentNum` _asbp_tpscharacter) 1) _asbp_tpscharacter)
    (`self.K2_DestroyActor`)
    (else
      (set `self.HitNum` (+ _hitnum 1))
      (if _returnvalue
        (`BlackboardComponent.SetValueAsBool` (`AIBlueprintHelperLibrary.GetBlackboard` self) "Ishit" _returnvalue)))))

(fn `UserConstructionScript`
  (`parent.UserConstructionScript`))